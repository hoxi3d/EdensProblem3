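; BP_BuildingMaster is a building Blueprint, named as the master class for the game's buildings.
; Its construction script applies DisplayMesh to the static mesh, then passes that mesh to helpers that set up the building's Entrance and Collision box.
; SetCalendar and SetClock are stubs that return false, and a node building a construction struct from the class, proxy and transform sits unused.
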(fn `SetCalendar`
  (params (Date :type "Array of Integer (by ref)"))
  (returns (Success :type Boolean))
  (return false))

(fn `SetClock`
  (params (Time :type "Array of Integer (by ref)"))
  (returns (Success :type Boolean))
  (return false))

(fn `UserConstructionScript`
  (`StaticMeshComponent.SetStaticMesh` (`self.StaticMesh`) (`self.DisplayMesh`))
  (`/Game/MechanicsandGears/Libraries/FunctionLibrary.SetBuildingEntrance` (`self.Entrance`) (`self.StaticMesh`))
  (`/Game/MechanicsandGears/Libraries/FunctionLibrary.SetBuildingCollisionBox` (`self.Collision`) (`self.StaticMesh`)))