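; Behavior tree task that checks an NPC in for a work shift at the construction proxy stored in its CurrentLocation blackboard key.
; With a valid location, it calls ReportToShift with the pawn, marks the NPC busy, hides it in game and finishes successfully.
; Without one, it clears the busy flag and fails, and both paths clear TargetLocation.
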(event `self.ReceiveExecuteAI`
  (params (OwnerController :type "AIController Object Reference") (ControlledPawn :type "Pawn Object Reference"))
  (bind _pawn (`self.Pawn`))
  (bind _returnvalue (`BTFunctionLibrary.GetBlackboardValueAsObject` (`self.CurrentLocation`)))
  (if (not (`KismetSystemLibrary.IsValid` (`self.Controller`)))
    (set `self.Controller` (cast `/Game/MechanicsandGears/Blueprints/Ai/NPC_AIController` OwnerController :!pure true)))
  (if (not (`KismetSystemLibrary.IsValid` (`self.Pawn`)))
    (set `self.Pawn` (cast `/Game/MechanicsandGears/Blueprints/Ai/BP_NPC` ControlledPawn :!pure true)))
  (`/Engine/EditorBlueprintResources/StandardMacros.IsValid` _returnvalue
    (:`Is Valid`
      (`/Game/MechanicsandGears/Blueprints/Construction/BP_ConstructionProxy.ReportToShift` (cast `/Game/MechanicsandGears/Blueprints/Construction/BP_ConstructionProxy` _returnvalue :!pure true) _pawn)
      (`BTFunctionLibrary.SetBlackboardValueAsBool` (`self.IsBusy`) true)
      (`Actor.SetActorHiddenInGame` _pawn true)
      (`BTFunctionLibrary.ClearBlackboardValue` (`self.TargetLocation`))
      (`self.FinishExecute` true))
    (:`Is Not Valid`
      (`BTFunctionLibrary.ClearBlackboardValue` (`self.TargetLocation`))
      (`BTFunctionLibrary.SetBlackboardValueAsBool` (`self.IsBusy`))
      (`self.FinishExecute` false))))