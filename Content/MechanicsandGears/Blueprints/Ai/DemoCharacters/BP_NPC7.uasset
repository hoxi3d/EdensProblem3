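; NPC character that gets a random name profile and shows its own HUD on request.
; Construction picks a name from gender-specific enums, with gender fixed to Male; the debug print rolls separately from the stored name.
; BeginPlay caches the AI controller, binds to the camera pawn controller's HUD request and creates the widget, which DisplayHUD shows when this NPC is targeted.
; SetIsBusy writes the AI blackboard's busy flag.
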(event Custom|DisplayHUD
  (params (Actor :type Actor%20Object%20Reference))
  (if (== Actor self)
    (UserInterface|Viewport|AddtoViewport (Variables|Default|GetNPC_HUD) 0)))

(event EventBeginPlay
  (Variables|Default|SetAIControllerRef (.AsNPC%20AIController (Utilities|Casting|CastToNPC_AIController (AI|GetAIController self))))
  (bind _asbp_my_cam_pawn_controller (Utilities|Casting|CastToBP_MyCamPawnController (Game|GetPlayerController 0)))
  (bind _output_get (Variables|Default|SetCamerPawnRef _asbp_my_cam_pawn_controller))
  (EventDispatchers|BindEventtoHUDRequest _output_get (EventDispatchers|CreateEvent :!event Custom|DisplayHUD))
  (bind _returnvalue (UserInterface|CreateWidget "/Game/MechanicsandGears/HUD/NPC_HUD.NPC_HUD_C"))
  (Variables|Default|SetNPC_HUD _returnvalue))

(fn ConstructionScript
  (CallFunction|RandomNPCFeatures))

(fn AnimInstance
  (return))

(fn RandomNPCFeatures
  (switch Utilities|FlowControl|Switch|SwitchonNPCGenderType_ENUM "NewEnumerator0"
    (:NewEnumerator0
      (bind _name (CallFunction|GetRandomName "NewEnumerator0"))
      (Variables|Default|SetMyProfile (Utilities|Struct|MakeNPCProfile_Struct _name "NewEnumerator0")))
    (:NewEnumerator1
      (bind _name_2 (CallFunction|GetRandomName "NewEnumerator1"))
      (Variables|Default|SetMyProfile (Utilities|Struct|MakeNPCProfile_Struct _name_2 "NewEnumerator1")))))

(fn GetRandomName
  (params (Gender :type NPCGenderType_ENUM%20Enum :default "NewEnumerator0"))
  (bind _returnvalue (|GetNumEnumEntries))
  (bind _returnvalue_2 (|GetNumEnumEntries))
  (bind _returnvalue_3 (- _returnvalue_2 1))
  (bind _returnvalue_4 (- _returnvalue 1))
  (bind _returnvalue_5 (Math|Random|RandomIntegerinRange 0 _returnvalue_3))
  (bind _returnvalue_6 (Math|Random|RandomIntegerinRange 0 _returnvalue_4))
  (bind _returnvalue_7 (Math|Conversions|ToByte(Integer) _returnvalue_5))
  (bind _returnvalue_8 (Math|Conversions|ToByte(Integer) _returnvalue_6))
  (bind _returnvalue_9 (Utilities|Enum|ByteToEnumNPCNameMale_ENUM _returnvalue_8))
  (bind _returnvalue_10 (Utilities|Enum|ByteToEnumNPCNameFemale_ENUM _returnvalue_7))
  (bind _returnvalue_11 (Utilities|String|EnumtoString _returnvalue_9))
  (bind _returnvalue_12 (Utilities|String|EnumtoString _returnvalue_10))
  (switch Utilities|FlowControl|Switch|SwitchonNPCGenderType_ENUM Gender
    (:NewEnumerator0
      (Development|PrintString _returnvalue_11)
      (return _returnvalue_11))
    (:NewEnumerator1
      (Development|PrintString _returnvalue_12)
      (return _returnvalue_12))))

(fn SetIsBusy
  (params (IsBusy :type Boolean))
  (AI|Components|Blackboard|SetValueasBool (AI|GetBlackboard (Variables|Default|GetAIControllerRef)) (Variables|Default|GetIsBusy) IsBusy)
  (return))