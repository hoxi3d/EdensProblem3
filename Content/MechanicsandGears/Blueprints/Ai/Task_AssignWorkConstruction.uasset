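; Behavior tree task that assigns an NPC construction work by targeting the first proxy in the construction manager's list.
; It reaches that manager through the AI controller's camera controller reference, using a macro to cast the controller and pawn.
; It writes the proxy's entrance location and the proxy itself to the TargetLocation and Destination blackboard keys, failing if no proxies exist.
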(event `self.ReceiveExecuteAI`
  (params (OwnerController :type "AIController Object Reference") (ControlledPawn :type "Pawn Object Reference"))
  (bind _proxies (`/Game/MechanicsandGears/Blueprints/Construction/BP_ConstructionManager.Proxies` (`/Game/MechanicsandGears/Blueprints/BP_MyCamPawnController.ConstructionManagerRef` (`/Game/MechanicsandGears/Blueprints/Ai/NPC_AIController.CameraControllerRef` (`self.Controller`)))))
  (bind _output (`|GetArrayItem` _proxies))
  (if (not (`KismetSystemLibrary.IsValid` (`self.Controller`)))
    (set `self.Controller` (cast `/Game/MechanicsandGears/Blueprints/Ai/NPC_AIController` OwnerController :!pure true)))
  (if (not (`KismetSystemLibrary.IsValid` (`self.Pawn`)))
    (set `self.Pawn` (cast `/Game/MechanicsandGears/Blueprints/Ai/BP_NPC` ControlledPawn :!pure true)))
  (if (> (`KismetArrayLibrary.Array_Length` _proxies) 0)
    (`BTFunctionLibrary.SetBlackboardValueAsVector` (`self.TargetLocation`) (`SceneComponent.K2_GetComponentLocation` (`/Game/MechanicsandGears/Blueprints/Construction/BP_ConstructionProxy.Entrance` _output)))
    (`BTFunctionLibrary.SetBlackboardValueAsObject` (`self.Destination`) _output)
    (`self.FinishExecute` true)
    (else
      (`self.FinishExecute` false))))