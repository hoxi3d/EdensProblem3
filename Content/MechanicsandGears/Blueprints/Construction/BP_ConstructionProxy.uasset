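; BP_ConstructionProxy is a ghost-material placeholder for a building under construction, with an entrance and collision box fitted to its display mesh.
; Workers register through ReportToShift, and Tick advances a work clock scaled by worker count and the game-speed time unit.
; When work time reaches the construction time, it signals completion, unhides and frees its workers, then destroys itself after a short delay.
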(event `self.ReceiveBeginPlay`
  ;[1 1 1] Game Speed/Begin Play
  (bind _output_get (set `self.GameStateRef` (cast `/Game/MechanicsandGears/GameBPs/BP_MyGameState` (`GameplayStatics.GetGameState`) :!pure true)))
  (add `/Game/MechanicsandGears/GameBPs/BP_MyGameState.UpdateGameSpeed` _output_get (`|CreateDelegate` :!event `AdjustTime`))
  (bind _time_unit (`/Game/MechanicsandGears/GameBPs/BP_MyGameState.GetCurrentTimeUnit` (`self.GameStateRef`)))
  (set `self.TimeUnit` _time_unit))

(event `self.ReceiveTick`
  (params (DeltaSeconds :type "Float (single-precision)"))
  ;[1 1 1] Do Work
  (set `self.Delta` DeltaSeconds)
  (if (not (`self.IsConstructionCompleted`))
    (`self.DoWork`)
    (if (>= (`self.WorkTimeSpent`) (`self.ConstructionTime`))
      (set `self.IsConstructionCompleted` true)
      (`self.ConstructionComplete` self)
      (`self.ConstructionCompleted`)
      (`KismetSystemLibrary.Delay` 0.2)
      (`self.K2_DestroyActor`))))

(event `AdjustTime`
  (params (TimeUnit :type "Float (double-precision)"))
  ;[1 1 1] Adjust Time
  (set `self.TimeUnit` TimeUnit))

(fn `ConstructionCompleted`
  (if (> (`self.GetWorkforce`) 0.0)
    (for _array_element (`self.ActiveWorkers`)
      (`/Game/MechanicsandGears/Blueprints/Ai/BP_NPC.SetIsBusy` _array_element false)
      (`self.SetActorHiddenInGame` _array_element false))
    (set `self.ActiveWorkers` (`|MakeArray` null :!type "/Game/MechanicsandGears/Blueprints/Ai/BP_NPC Object Reference"))
    (return)
    (else
      (return))))

(fn `DoWork`
  (bind _activeworkers (`self.GetWorkforce`))
  (if (> _activeworkers 0.0)
    (bind _output_get (set `self.ClockWork` (`/Game/MechanicsandGears/Libraries/FunctionLibrary.SetClockWork` (`self.Delta`) (/ (`self.TimeUnit`) _activeworkers) (`self.ClockWork`))))
    (set `self.WorkTimeSpent` (* _output_get 60.0))
    (return)
    (else
      (return))))

(fn `GetWorkforce`
  (returns (ActiveWorkers :type "Float (double-precision)"))
  (return (`KismetMathLibrary.Conv_IntToDouble` (`KismetArrayLibrary.Array_Length` (`self.ActiveWorkers`)))))

(fn `ReportToShift`
  (params (Worker :type "/Game/MechanicsandGears/Blueprints/Ai/BP_NPC Object Reference"))
  (`KismetArrayLibrary.Array_Add` (`self.ActiveWorkers`) Worker)
  (return))

(fn `SetConstructionTime`
  (params (WorkHours :type "Float (double-precision)"))
  (set `self.ConstructionTime` (* WorkHours 60.0))
  (return))

(fn `UserConstructionScript`
  (bind _staticmesh (`self.StaticMesh`))
  (`StaticMeshComponent.SetStaticMesh` _staticmesh (`self.DisplayMesh`))
  (`PrimitiveComponent.SetMaterial` _staticmesh 0 "/Game/ArtAssets/MasterMaterials/MM_GhostMaterial.MM_GhostMaterial")
  (`/Game/MechanicsandGears/Libraries/FunctionLibrary.SetBuildingEntrance` (`self.Entrance`) (`self.StaticMesh`))
  (`/Game/MechanicsandGears/Libraries/FunctionLibrary.SetBuildingCollisionBox` (`self.Collision`) (`self.StaticMesh`)))