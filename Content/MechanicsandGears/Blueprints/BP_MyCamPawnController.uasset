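; Player controller for a building game, handling camera navigation, object selection and building placement.
; On BeginPlay it spawns the construction manager and ghost building, then creates the main HUD.
; In build mode the ghost follows the cursor and rotates, and clicking queues its construction; otherwise clicks send hit actors to the HUD.
; It drives the camera pawn with zoom-scaled movement, screen-edge scrolling, gated mouse panning and spring-arm zoom, plus a temporary NPC spawn key.
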(event `self.ReceiveTick`
  (params (DeltaSeconds :type "Float (single-precision)"))
  (bind _cube (`self.Cube`))
  (bind (_returnvalue_x _returnvalue_y _returnvalue_z) (`KismetMathLibrary.BreakVector` (`SceneComponent.K2_GetComponentLocation` _cube)))
  ;[1 1 1] SetCursorWorldPosition
  (if (`self.BuildModeActive`)
    (`SceneComponent.K2_SetWorldLocation` _cube (`KismetMathLibrary.MakeVector` (+ _returnvalue_x (* (`self.GetInputAxisKeyValue`) 50.0)) _returnvalue_y (+ _returnvalue_z (* (`self.GetInputAxisKeyValue`) 50.0))) false false)
    (if (!= (`self.GhostBuildingRef`) null)
      (`/Game/MechanicsandGears/Blueprints/Buildings/BP_GhostBuilding.SetCursorPosition` (`self.GhostBuildingRef`) (`/Game/MechanicsandGears/Libraries/FunctionLibrary.SetCursorWorldPosition` self (`self.SetSightDistance`))))))

(event `Key|LeftMouseButton`
  (params (Key :type "Key Structure"))
  (bind (_bblockinghit _binitialoverlap _time _distance _location _impactpoint _normal _impactnormal _physmat _hitactor) (`GameplayStatics.BreakHitResult` (`self.GetHitResultUnderCursorForObjects` (`self.SelectableObjects_ENUM`))))
  ;[1 1 1] Left Click Build
  (:`Pressed`
    (if (`self.BuildModeActive`)
      (if (and (`self.BuildModeActive`) (not (`/Game/MechanicsandGears/Blueprints/Buildings/BP_GhostBuilding.GetIsOverlapping` (`self.GhostBuildingRef`))))
        (bind _constructionstruct (`/Game/MechanicsandGears/Blueprints/Buildings/BP_GhostBuilding.GetConstructionStruct` (`self.GhostBuildingRef`)))
        (`/Game/MechanicsandGears/Blueprints/Construction/BP_ConstructionManager.QueueConstruction` (`self.ConstructionManagerRef`) _constructionstruct)
        (`/Game/MechanicsandGears/Blueprints/Buildings/BP_GhostBuilding.KillGhost` (`self.GhostBuildingRef`)))
      (elif (!= _hitactor null)
        (`self.HUDRequest` _hitactor)))))

(event `InputAction|RotateBuildingRight`
  (params (Key :type "Key Structure"))
  (bind _ghostbuildingref (`self.GhostBuildingRef`))
  ;[1 1 1] Rotate Building
  (:`Pressed`
    (if (and (`KismetSystemLibrary.IsValid` _ghostbuildingref) (`self.BuildModeActive`))
      (`self.K2_SetActorRotation` _ghostbuildingref (`KismetMathLibrary.MakeRotator` (.roll (`self.K2_GetActorRotation` _ghostbuildingref)) (.pitch (`self.K2_GetActorRotation` _ghostbuildingref)) (- (.yaw (`self.K2_GetActorRotation` _ghostbuildingref)) (`self.BuildingRotationRate`))) false))))

(event `self.ReceiveBeginPlay`
  (bind _returnvalue (`KismetMathLibrary.MakeTransform` (0.0 0.0 0.0)))
  ;[1 1 1] Begin Play
  (`|ExecutionSequence`
    (:`then_0`
      (`self.ReferenceCasts`))
    (:`then_1`
      (bind _returnvalue_2 (`|SpawnActorFromClass` "/Game/MechanicsandGears/Blueprints/Construction/BP_ConstructionManager.BP_ConstructionManager_C" _returnvalue "AlwaysSpawn" "OverrideRootScale" null null))
      (set `self.ConstructionManagerRef` _returnvalue_2))
    (:`then_2`
      (bind _returnvalue_3 (`|SpawnActorFromClass` "/Game/MechanicsandGears/Blueprints/Buildings/BP_GhostBuilding.BP_GhostBuilding_C" _returnvalue "AlwaysSpawn" "OverrideRootScale" null self (0.0 0.0 0.0) null))
      (set `self.GhostBuildingRef` _returnvalue_3))
    (:`then_3`
      (`WidgetBlueprintLibrary.SetInputMode_GameAndUIEx` null null "LockAlways" false)
      (`self.CreateHUDs`)
      (`UserWidget.AddToViewport` (`self.MainHud_Ref`) 0))))

(event `InputAction|RotateBuildingLeft`
  (params (Key :type "Key Structure"))
  (bind _ghostbuildingref (`self.GhostBuildingRef`))
  ;[1 1 1] Rotate Building
  (:`Pressed`
    (if (and (`KismetSystemLibrary.IsValid` _ghostbuildingref) (`self.BuildModeActive`))
      (`self.K2_SetActorRotation` _ghostbuildingref (`KismetMathLibrary.MakeRotator` (.roll (`self.K2_GetActorRotation` _ghostbuildingref)) (.pitch (`self.K2_GetActorRotation` _ghostbuildingref)) (+ (.yaw (`self.K2_GetActorRotation` _ghostbuildingref)) (`self.BuildingRotationRate`))) false))))

(event `Key|V`
  (params (Key :type "Key Structure"))
  (bind (_location_x _location_y) (`KismetMathLibrary.BreakVector` (`/Game/MechanicsandGears/Libraries/FunctionLibrary.SetCursorWorldPosition` self 10000.0)))
  ;[1 1 1] TempSpawn
  (:`Pressed`
    (`|SpawnActorFromClass` "/Game/MechanicsandGears/Blueprints/Ai/BP_NPC.BP_NPC_C" (`KismetMathLibrary.MakeTransform` (`KismetMathLibrary.MakeVector` _location_x _location_y 50.0)) "Undefined" "OverrideRootScale" null null)))

(event `InputAxis|MoveForward`
  (params (AxisValue :type "Float (single-precision)"))
  (bind _camerapawnref (`self.CameraPawnRef`))
  ;[1 1 1] MovementX
  (if (not (`self.DisableCamNav`))
    (`self.K2_SetActorTransform` _camerapawnref (`self.MovementX` (`self.MovementSpeedCalc`) (`self.FastMoveMult`) AxisValue _camerapawnref) false false)))

(event `InputAxis|MoveRight`
  (params (AxisValue :type "Float (single-precision)"))
  (bind _camerapawnref (`self.CameraPawnRef`))
  ;[1 1 1] MovementY
  (if (not (`self.DisableCamNav`))
    (`self.K2_SetActorTransform` _camerapawnref (`KismetMathLibrary.MakeTransform` (`KismetMathLibrary.MakeVector` (.x (.location (`self.MovementY` (`self.MovementSpeedCalc`) (`self.FastMoveMult`) AxisValue _camerapawnref))) (.y (.location (`self.MovementY` (`self.MovementSpeedCalc`) (`self.FastMoveMult`) AxisValue _camerapawnref))) 500.0) (.rotation (`self.MovementY` (`self.MovementSpeedCalc`) (`self.FastMoveMult`) AxisValue _camerapawnref)) (.scale (`self.MovementY` (`self.MovementSpeedCalc`) (`self.FastMoveMult`) AxisValue _camerapawnref))) false false)))

(event `InputAction|PanReset`
  (params (Key :type "Key Structure"))
  (bind _camerapawnref (`self.CameraPawnRef`))
  ;[1 1 1] PanReset
  (:`Pressed`
    (`self.K2_SetActorRotation` _camerapawnref (`KismetMathLibrary.MakeRotator` (.roll (`self.K2_GetActorRotation` _camerapawnref)) 0.0 (.yaw (`self.K2_GetActorRotation` _camerapawnref))) false)))

(event `InputAxisKey|MouseX`
  (params (AxisValue :type "Float (single-precision)"))
  (bind _camerapawnref (`self.CameraPawnRef`))
  ;[1 1 1] Pan X
  (`/Engine/EditorBlueprintResources/StandardMacros.Gate` true :!label _label
    (:`Exit`
      (`self.K2_SetActorRotation` _camerapawnref (`KismetMathLibrary.MakeRotator` (.roll (`self.K2_GetActorRotation` _camerapawnref)) (.pitch (`self.K2_GetActorRotation` _camerapawnref)) (+ (.yaw (`self.K2_GetActorRotation` _camerapawnref)) (* (`self.PanSense`) AxisValue))) false))))

(event `InputAction|Pan`
  (params (Key :type "Key Structure"))
  ;[1 1 1] Pan X
  (:`Pressed`
    (goto _label :!via `Open`))
  (:`Released`
    (goto _label :!via `Close`)))

(event `InputAxisKey|MouseY`
  (params (AxisValue :type "Float (single-precision)"))
  (bind _camerapawnref (`self.CameraPawnRef`))
  ;[1 1 1] Pan Y
  (`/Engine/EditorBlueprintResources/StandardMacros.Gate` true :!label _label_2
    (:`Exit`
      (`self.K2_SetActorRotation` _camerapawnref (`KismetMathLibrary.MakeRotator` (.roll (`self.K2_GetActorRotation` _camerapawnref)) (`KismetMathLibrary.FClamp` (+ (.pitch (`self.K2_GetActorRotation` _camerapawnref)) (* (`self.PanSense`) AxisValue)) -15.0 45.0) (.yaw (`self.K2_GetActorRotation` _camerapawnref))) false))))

(event `InputAction|Pan`
  (params (Key :type "Key Structure"))
  ;[1 1 1] Pan Y
  (:`Pressed`
    (set `self.DisableCamNav` false)
    (goto _label_2 :!via `Open`))
  (:`Released`
    (set `self.DisableCamNav` false)
    (goto _label_2 :!via `Close`)))

(event `Key|LeftShift`
  (params (Key :type "Key Structure"))
  ;[1 1 1] SpeedMult
  (:`Pressed`
    (set `self.FastMoveMult` 3.0))
  (:`Released`
    (set `self.FastMoveMult` 1.0)))

(event `InputAxisKey|MouseX`
  (params (AxisValue :type "Float (single-precision)"))
  ;[1 1 1] EdgeMovement
  (if (not (`self.DisableCamNav`))
    (bind (_deltaxspeed _deltayspeed) (`self.ScreenEdgeScroll` :!label _label_3))
    (`self.K2_AddActorLocalOffset` (`self.CameraPawnRef`) (`KismetMathLibrary.MakeVector` _deltaxspeed _deltayspeed) true false)))

(event `InputAction|ZoomIn`
  (params (Key :type "Key Structure"))
  (bind _springarm (`/Game/MechanicsandGears/Blueprints/BP_MyCameraPawn.SpringArm` (`self.CameraPawnRef`)))
  ;[1 1 1] ZoomIn/Out
  (:`Pressed`
    (set `SpringArmComponent.TargetArmLength` (`KismetMathLibrary.FClamp` (- (`SpringArmComponent.TargetArmLength` _springarm) (`self.ZoomSense`)) 500.0 (`self.MaxArmDist`)) _springarm)))

(event `InputAxisKey|MouseY`
  (params (AxisValue :type "Float (single-precision)"))
  ;[1 1 1] EdgeMovement
  (if (not (`self.DisableCamNav`))
    (goto _label_3 :!via `MouseY`)))

(event `InputAction|ZoomOut`
  (params (Key :type "Key Structure"))
  (bind _springarm (`/Game/MechanicsandGears/Blueprints/BP_MyCameraPawn.SpringArm` (`self.CameraPawnRef`)))
  ;[1 1 1] ZoomIn/Out
  (:`Pressed`
    ;[1 1 1] ZoomReset
    (set `SpringArmComponent.TargetArmLength` (`KismetMathLibrary.FClamp` (+ (`self.ZoomSense`) (`SpringArmComponent.TargetArmLength` _springarm)) 500.0 (`self.MaxArmDist`)) _springarm)))

(event `InputAction|ZoomReset`
  (params (Key :type "Key Structure"))
  ;[1 1 1] ZoomReset
  (:`Pressed`
    (set `SpringArmComponent.TargetArmLength` 1500.0 (`/Game/MechanicsandGears/Blueprints/BP_MyCameraPawn.SpringArm` (`self.CameraPawnRef`)))))

(event `InputAction|Deselect`
  (params (Key :type "Key Structure"))
  ;[1 1 1] Deselect
  (:`Pressed`
    (if (`self.BuildModeActive`)
      (`/Game/MechanicsandGears/Blueprints/Buildings/BP_GhostBuilding.KillGhost` (`self.GhostBuildingRef`))
      (set `self.BuildModeActive` false))))

(fn `MovementSpeedCalc`
  (returns (MovementSensitivity :type "Float (double-precision)"))
  (return (`KismetMathLibrary.FClamp` (/ (`SpringArmComponent.TargetArmLength` (`/Game/MechanicsandGears/Blueprints/BP_MyCameraPawn.SpringArm` (`self.CameraPawnRef`))) 100.0) 5.0 20.0)))

(fn `SetCalendar`
  (params (Date :type "Array of Integer (by ref)"))
  (returns (Success :type Boolean))
  (return false))

(fn `SetClock`
  (params (Time :type "Array of Integer (by ref)"))
  (returns (Success :type Boolean))
  (return false))

(fn `SetSightDistance`
  (returns (SightDistance :type "Float (double-precision)"))
  (return (+ (`self.SightDistance`) (`SpringArmComponent.TargetArmLength` (`/Game/MechanicsandGears/Blueprints/BP_MyCameraPawn.SpringArm` (`self.CameraPawnRef`))))))

(fn `UserConstructionScript`)