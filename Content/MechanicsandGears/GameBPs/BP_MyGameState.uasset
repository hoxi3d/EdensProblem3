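; Game state Blueprint that runs the in-game clock, calendar and game speed.
; Each Tick advances a ClockWork value by the current TimeUnit, derives hours, minutes and seconds, rolls days into months and years, and pushes both to the player controller's main HUD.
; Speed updates scale the default TimeUnit by a multiplier and broadcast it through UpdateGameSpeed.
; SetClock and SetCalendar are stubs returning false.
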(event `self.ReceiveBeginPlay`
  ;[1 1 1] Clock and Calendar
  (bind _asbp_my_cam_pawn_controller (cast `/Game/MechanicsandGears/Blueprints/BP_MyCamPawnController` (`GameplayStatics.GetPlayerController` 0)))
  (set `self.ControllerRef` _asbp_my_cam_pawn_controller)
  (set `self.ClockWork` (+ (`KismetMathLibrary.Conv_IntToDouble` (`self.Hours`)) (`KismetMathLibrary.Conv_IntToDouble` (`self.Minutes`)) (`KismetMathLibrary.Conv_IntToDouble` (`self.Seconds`))))
  (set `self.GameDate` (`|MakeArray` (`self.Day`) (`self.Month`) (`self.Year`)))
  (set `self.MainUIRef` (`/Game/MechanicsandGears/Blueprints/BP_MyCamPawnController.MainHud_Ref` (`self.ControllerRef`)))
  (set `self.TimeUnit` (`self.DefaultGameSpeed`)))

(event `self.ReceiveTick`
  (params (DeltaSeconds :type "Float (single-precision)"))
  (bind (_clockworkout _daytick) (`/Game/MechanicsandGears/Libraries/FunctionLibrary.SetClockWork` DeltaSeconds (`self.TimeUnit`) (`self.ClockWork`)))
  ;[1 1 1] Clock and Calendar
  (set `self.ClockWork` _clockworkout)
  (set `self.DayTick` _daytick)
  (`self.Clock`)
  (`self.Calendar`))

(event `/Game/MechanicsandGears/Interfaces/I_HUD.UpdateGameStateSpeed`
  (params (Multiplier :type "Float (single-precision)"))
  ;[1 1 1] GameSpeed
  (bind _output_get (set `self.TimeUnit` (* (`self.DefaultGameSpeed`) Multiplier)))
  (`self.UpdateGameSpeed` _output_get))

(fn `Calendar`
  (bind _output_get (set `self.Day` (+ (`self.Day`) (`self.DayTick`))))
  (if (> _output_get (`KismetMathLibrary.DaysInMonth` (`self.Year`) (`self.Month`)))
    (set `self.Day` 0)
    (set `self.Month` (+ (`self.Month`) 1)))
  (if (> (`self.Month`) 12)
    (bind _output_get_2 (set `self.Month` 1))
    (set `self.Year` (+ _output_get_2 (`self.Year`))))
  (bind _output_get_3 (set `self.GameDate` (`|MakeArray` (`self.Day`) (`self.Month`) (`self.Year`))))
  (message `/Game/MechanicsandGears/Interfaces/I_HUD.SetCalendar` (`/Game/MechanicsandGears/Blueprints/BP_MyCamPawnController.MainHud_Ref` (`self.ControllerRef`)) _output_get_3))

(fn `Clock`
  (bind (_remainder _returnvalue) (`KismetMathLibrary.FMod` (* (`self.ClockWork`) 3600.0) 60.0))
  (bind (_remainder_2 _returnvalue_2) (`KismetMathLibrary.FMod` (`KismetMathLibrary.Conv_IntToDouble` _returnvalue) 60.0))
  (set `self.Seconds` (`KismetMathLibrary.FFloor` _remainder))
  (set `self.Minutes` (`KismetMathLibrary.FFloor` _remainder_2))
  (set `self.Hours` (`KismetMathLibrary.FFloor` (`KismetMathLibrary.FMod` (`KismetMathLibrary.Conv_IntToDouble` _returnvalue_2) 24.0)))
  (bind _output_get (set `self.GameTime` (`|MakeArray` (`self.Seconds`) (`self.Minutes`) (`self.Hours`))))
  (message `/Game/MechanicsandGears/Interfaces/I_HUD.SetClock` (`/Game/MechanicsandGears/Blueprints/BP_MyCamPawnController.MainHud_Ref` (`self.ControllerRef`)) _output_get))

(fn `GetCurrentTimeUnit`
  (returns (`Time Unit` :type "Float (double-precision)"))
  (return (`self.TimeUnit`)))

(fn `SetCalendar`
  (params (Date :type "Array of Integer (by ref)"))
  (returns (Success :type Boolean))
  (return false))

(fn `SetClock`
  (params (Time :type "Array of Integer (by ref)"))
  (returns (Success :type Boolean))
  (return false))

(fn `UserConstructionScript`)